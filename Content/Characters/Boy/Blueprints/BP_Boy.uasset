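; Player Boy character with camera-relative movement, interact, jump and cancel actions, scripted move-then-rotate, and a light-dependent material form.
; Tick calls SetSocketsLightState, feeds heart values from the Boy_Sockets parameter collection to Niagara, and shrinks the capsule outside material form.
; SetBonesLightState, uncalled here, tests bones and heart against BP_UnreachableLight beams using line distance and visibility traces.
; It stores each bone's nearest light and derives material form from the heart.
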(event `InputAxis|Move Forward / Backward`
  (params (AxisValue :type "Float (single-precision)"))
  (if (`|EnumEquality` (`self.CharacterPositionState`) "NewEnumerator0")
    (bind (_direction _scalevalue) (`self.GetUpDownMovementDirection` AxisValue))
    (`self.AddMovementInput` _direction _scalevalue)))

(event `InputAxis|Move Right / Left`
  (params (AxisValue :type "Float (single-precision)"))
  (if (`|EnumEquality` (`self.CharacterPositionState`) "NewEnumerator0")
    (bind (_direction _scalevalue) (`self.GetRightLeftMovementDirection` AxisValue))
    (`self.AddMovementInput` _direction _scalevalue)))

(event `self.ReceiveBeginPlay`
  (`KismetMaterialLibrary.SetScalarParameterValue` "/Game/GeneralMaterials/Lights/Boy_Sockets.Boy_Sockets" "IsEditor" -1.0)
  (`PlayerController.SetAudioListenerOverride` :`self` (`GameplayStatics.GetPlayerController` 0) :`AttachToComponent` (`self.Mesh`))
  (`ActorComponent.Activate` (`self.NS_Boy`) false)
  (set `self.CapsuleRadius` (`CapsuleComponent.GetUnscaledCapsuleRadius` (`self.CapsuleComponent`))))

(event `self.ReceiveTick`
  (params (DeltaSeconds :type "Float (single-precision)"))
  (bind _ns_boy (`self.NS_Boy`))
  (bind _capsulecomponent (`self.CapsuleComponent`))
  (bind _bisinmaterialform (`self.bIsInMaterialForm`))
  (`self.SetSocketsLightState` "/Game/GeneralMaterials/Lights/Boy_Sockets.Boy_Sockets")
  (bind _returnvalue (`KismetMaterialLibrary.GetVectorParameterValue` "/Game/GeneralMaterials/Lights/Boy_Sockets.Boy_Sockets" "HeartPos"))
  (`FXSystemComponent.SetVectorParameter` _ns_boy "HeartPos" (`KismetMathLibrary.Conv_LinearColorToVector` _returnvalue))
  (bind _returnvalue_2 (`KismetMaterialLibrary.GetScalarParameterValue` "/Game/GeneralMaterials/Lights/Boy_Sockets.Boy_Sockets" "HeartAlpha"))
  (`FXSystemComponent.SetFloatParameter` _ns_boy "HeartAlpha" _returnvalue_2)
  (`FXSystemComponent.SetBoolParameter` _ns_boy "HeartLighted" _bisinmaterialform)
  (if _bisinmaterialform
    (`CapsuleComponent.SetCapsuleRadius` _capsulecomponent (`self.CapsuleRadius`) true)
    (else
      (`CapsuleComponent.SetCapsuleRadius` _capsulecomponent 5.0 true))))

(event `InputAction|Action`
  (params (Key :type "Key Structure"))
  (:`Pressed`
    (`self.InteractAction`)))

(event `InputAction|Jump`
  (params (Key :type "Key Structure"))
  (:`Pressed`
    (`self.JumpAction`)))

(event `InputAction|Cancel`
  (params (Key :type "Key Structure"))
  (:`Pressed`
    (`self.CancelAction`)))

(event `CheckMoveEnd`
  ;[1 1 1] Boy move to function override
  (`self.CheckIfHasMoveToEnded` (.location (stale `self.MoveCharacterTo` DestinationTransform))))

(event `self.MoveCharacterTo`
  (params (DestinationTransform :type "Transform Structure"))
  ;[1 1 1] Boy move to function override
  (`AIBlueprintHelperLibrary.SimpleMoveToLocation` (`GameplayStatics.GetPlayerController` 0) DestinationTransform_Location)
  (add `self.FMoveToEndedEvent` (delegate `RotateTo`))
  (bind _returnvalue (`KismetSystemLibrary.K2_SetTimerDelegate` (delegate `CheckMoveEnd`) 0.001 true))
  (set `self.MovementTimerHandle` _returnvalue))

(event `RotateTo`
  ;[1 1 1] Boy move to function override
  (bind (_direction _alpha) (`Timeline|Rotate`)
    (:`Update`
      (`self.K2_SetActorRotation` (`KismetMathLibrary.RLerp` (`self.K2_GetActorRotation`) (.rotation (stale `self.MoveCharacterTo` DestinationTransform)) _alpha)))))

(fn `Get Light Info at Bone Pos`
  (params (BonePos :type "Vector Structure") (LightActor :type "Actor Object Reference"))
  (returns (IsLighted :type Boolean) (LightAxis :type "Vector Structure") (LightPos :type "Vector Structure") (LightAngle :type "Float (double-precision)") (LightRadius :type "Float (double-precision)"))
  (bind _returnvalue (`self.GetActorForwardVector` LightActor))
  (bind _returnvalue_2 (`self.K2_GetActorLocation` LightActor))
  (bind _asbp_unreachable_light (cast `/Game/GeneralBlueprints/BP_UnreachableLight` LightActor))
  (if (and (`UnreachableLight.bIsActive` _asbp_unreachable_light) (<= (`KismetMathLibrary.GetPointDistanceToLine` BonePos _returnvalue_2 _returnvalue) (`UnreachableLight.LightRadius` _asbp_unreachable_light)))
    (bind (_outhit _returnvalue_3) (`KismetSystemLibrary.LineTraceSingle` BonePos _returnvalue_2 "TraceTypeQuery1" false (`|MakeArray` _asbp_unreachable_light (`self.GetParentActor` _asbp_unreachable_light) null :!type "Actor Object Reference") "None" true (struct :`R` 1.0 :`A` 1.0) (struct :`G` 1.0 :`A` 1.0) 1.0))
    (return (not _returnvalue_3) _returnvalue _returnvalue_2 (`UnreachableLight.LightAngle` _asbp_unreachable_light) (`UnreachableLight.LightRadius` _asbp_unreachable_light))
    (else
      (return false (0.0 0.0 0.0) (0.0 0.0 0.0) 0.0 0.0))))

(fn `Get Light Info at Heart`
  (params (BonePos :type "Vector Structure") (LightActor :type "Actor Object Reference"))
  (returns (IsLighted :type Boolean) (LightAxis :type "Vector Structure") (LightPos :type "Vector Structure") (LightAngle :type "Float (double-precision)") (LightRadius :type "Float (double-precision)"))
  (bind _returnvalue (`self.K2_GetActorLocation` LightActor))
  (bind _asbp_unreachable_light (cast `/Game/GeneralBlueprints/BP_UnreachableLight` LightActor))
  (bind _lightradius (`UnreachableLight.LightRadius` _asbp_unreachable_light))
  (if (and (`UnreachableLight.bIsActive` _asbp_unreachable_light) (<= (`KismetMathLibrary.GetPointDistanceToLine` BonePos _returnvalue (`self.GetActorForwardVector` LightActor)) _lightradius))
    (bind (_outhit _returnvalue_2) (`KismetSystemLibrary.LineTraceSingle` BonePos _returnvalue "TraceTypeQuery1" false (`|MakeArray` _asbp_unreachable_light (`self.GetParentActor` _asbp_unreachable_light) (`self.InteractRegion`) (`self.JumpRegion`) self :!type "Actor Object Reference") "None" true (struct :`R` 1.0 :`A` 1.0) (struct :`G` 1.0 :`A` 1.0) 1.0))
    (return (not _returnvalue_2) (0.0 0.0 0.0) _returnvalue 0.0 _lightradius)
    (else
      (return false (0.0 0.0 0.0) (0.0 0.0 0.0) 0.0 0.0))))

(fn `GetRightLeftMovementDirection`
  (params (AxisValue :type "Float (double-precision)"))
  (returns (Direction :type "Vector Structure") (ScaleValue :type "Float (double-precision)"))
  (bind _returnvalue (`self.GetInputAxisValue`))
  (bind _returnvalue_2 (`KismetMathLibrary.Sqrt` (+ (* _returnvalue _returnvalue) (* AxisValue AxisValue))))
  (bind _returnvalue_3 (* AxisValue (`KismetMathLibrary.Normal` (`KismetMathLibrary.ProjectVectorOnToPlane` (`self.GetActorRightVector` (`GameplayStatics.GetPlayerCameraManager` 0)) (`self.GetActorUpVector`)))))
  (if (> _returnvalue_2 0.25)
    (if (== (`KismetMathLibrary.Abs` AxisValue) 1.0)
      (return (/ _returnvalue_3 _returnvalue_2) (- 1.0 (`self.GetInputAxisValue`)))
      (else
        (return _returnvalue_3 1.0)))
    (else
      (return (0.0 0.0 0.0) 0.0))))

(fn `GetUpDownMovementDirection`
  (params (AxisValue :type "Float (double-precision)"))
  (returns (Direction :type "Vector Structure") (ScaleValue :type "Float (double-precision)"))
  (bind _returnvalue (`self.GetInputAxisValue`))
  (bind _returnvalue_2 (`KismetMathLibrary.Sqrt` (+ (* _returnvalue _returnvalue) (* AxisValue AxisValue))))
  (bind _returnvalue_3 (* AxisValue (`KismetMathLibrary.Normal` (`KismetMathLibrary.ProjectVectorOnToPlane` (`self.GetActorForwardVector` (`GameplayStatics.GetPlayerCameraManager` 0)) (`self.GetActorUpVector`)))))
  (if (> _returnvalue_2 0.25)
    (if (== (`KismetMathLibrary.Abs` AxisValue) 1.0)
      (return (/ _returnvalue_3 _returnvalue_2) (- 1.0 (`self.GetInputAxisValue`)))
      (else
        (return _returnvalue_3 1.0)))
    (else
      (return (0.0 0.0 0.0) 0.0))))

(fn `Set Bones Light State`
  (locals (NLightedBones :type Integer) (IsHeartLighted :type Boolean) (HeartAlpha :type "Float (double-precision)") (HeartPos :type "Vector Structure"))
  (bind _lights (`self.Lights`))
  (bind _ns_boy (`self.NS_Boy`))
  (bind _lights_2 (`self.Lights`))
  (bind _capsulecomponent (`self.CapsuleComponent`))
  (bind _isheartlighted (`local.IsHeartLighted`))
  (bind _returnvalue (`SceneComponent.GetSocketLocation` (`self.Mesh`) "lowerarm_l"))
  (bind _returnvalue_2 (`SceneComponent.GetSocketLocation` (`self.Mesh`) "head"))
  (bind _returnvalue_3 (`SceneComponent.GetSocketLocation` (`self.Mesh`) "ball_r"))
  (bind _returnvalue_4 (`SceneComponent.GetSocketLocation` (`self.Mesh`) "ball_l"))
  (bind _returnvalue_5 (`SceneComponent.GetSocketLocation` (`self.Mesh`) "lowerarm_r"))
  (bind _returnvalue_6 (`SceneComponent.GetSocketLocation` (`self.Mesh`) "spine_02"))
  (bind _returnvalue_7 (`SceneComponent.GetSocketLocation` (`self.Mesh`) "hand_r"))
  (bind _returnvalue_8 (`SceneComponent.GetSocketLocation` (`self.Mesh`) "hand_l"))
  (bind _returnvalue_9 (`SceneComponent.GetSocketLocation` (`self.Mesh`) "calf_r"))
  (bind _returnvalue_10 (`SceneComponent.GetSocketLocation` (`self.Mesh`) "calf_l"))
  (set `local.NLightedBones` 0)
  (`KismetMaterialLibrary.SetVectorParameterValue` "/Game/GeneralMaterials/Lights/Boy_Sockets.Boy_Sockets" "HandR" (`KismetMathLibrary.Conv_VectorToLinearColor` _returnvalue_7))
  (`KismetMaterialLibrary.SetScalarParameterValue` "/Game/GeneralMaterials/Lights/Boy_Sockets.Boy_Sockets" "HandR_Light" -1.0)
  (`KismetMaterialLibrary.SetVectorParameterValue` "/Game/GeneralMaterials/Lights/Boy_Sockets.Boy_Sockets" "HandR" (`KismetMathLibrary.Conv_VectorToLinearColor` _returnvalue_8))
  (`KismetMaterialLibrary.SetScalarParameterValue` "/Game/GeneralMaterials/Lights/Boy_Sockets.Boy_Sockets" "HandL_Light" -1.0)
  (`KismetMaterialLibrary.SetVectorParameterValue` "/Game/GeneralMaterials/Lights/Boy_Sockets.Boy_Sockets" "ArmR" (`KismetMathLibrary.Conv_VectorToLinearColor` _returnvalue_5))
  (`KismetMaterialLibrary.SetScalarParameterValue` "/Game/GeneralMaterials/Lights/Boy_Sockets.Boy_Sockets" "ArmR_Light" -1.0)
  (`KismetMaterialLibrary.SetVectorParameterValue` "/Game/GeneralMaterials/Lights/Boy_Sockets.Boy_Sockets" "ArmL" (`KismetMathLibrary.Conv_VectorToLinearColor` _returnvalue))
  (`KismetMaterialLibrary.SetScalarParameterValue` "/Game/GeneralMaterials/Lights/Boy_Sockets.Boy_Sockets" "ArmL_Light" -1.0)
  (`KismetMaterialLibrary.SetVectorParameterValue` "/Game/GeneralMaterials/Lights/Boy_Sockets.Boy_Sockets" "Torso" (`KismetMathLibrary.Conv_VectorToLinearColor` _returnvalue_6))
  (`KismetMaterialLibrary.SetScalarParameterValue` "/Game/GeneralMaterials/Lights/Boy_Sockets.Boy_Sockets" "Torso_Light" -1.0)
  (`KismetMaterialLibrary.SetVectorParameterValue` "/Game/GeneralMaterials/Lights/Boy_Sockets.Boy_Sockets" "Head" (`KismetMathLibrary.Conv_VectorToLinearColor` _returnvalue_2))
  (`KismetMaterialLibrary.SetScalarParameterValue` "/Game/GeneralMaterials/Lights/Boy_Sockets.Boy_Sockets" "Head_Light" -1.0)
  (`KismetMaterialLibrary.SetVectorParameterValue` "/Game/GeneralMaterials/Lights/Boy_Sockets.Boy_Sockets" "LegR" (`KismetMathLibrary.Conv_VectorToLinearColor` _returnvalue_9))
  (`KismetMaterialLibrary.SetScalarParameterValue` "/Game/GeneralMaterials/Lights/Boy_Sockets.Boy_Sockets" "LegR_Light" -1.0)
  (`KismetMaterialLibrary.SetVectorParameterValue` "/Game/GeneralMaterials/Lights/Boy_Sockets.Boy_Sockets" "LegL" (`KismetMathLibrary.Conv_VectorToLinearColor` _returnvalue_10))
  (`KismetMaterialLibrary.SetScalarParameterValue` "/Game/GeneralMaterials/Lights/Boy_Sockets.Boy_Sockets" "LegL_Light" -1.0)
  (`KismetMaterialLibrary.SetVectorParameterValue` "/Game/GeneralMaterials/Lights/Boy_Sockets.Boy_Sockets" "FootR" (`KismetMathLibrary.Conv_VectorToLinearColor` _returnvalue_3))
  (`KismetMaterialLibrary.SetScalarParameterValue` "/Game/GeneralMaterials/Lights/Boy_Sockets.Boy_Sockets" "FootR_Light" -1.0)
  (`KismetMaterialLibrary.SetVectorParameterValue` "/Game/GeneralMaterials/Lights/Boy_Sockets.Boy_Sockets" "FootL" (`KismetMathLibrary.Conv_VectorToLinearColor` _returnvalue_4))
  (`KismetMaterialLibrary.SetScalarParameterValue` "/Game/GeneralMaterials/Lights/Boy_Sockets.Boy_Sockets" "FootL_Light" -1.0)
  (if (not (`KismetArrayLibrary.Array_IsEmpty` _lights_2))
    (for _array_element _lights_2
      (if (`KismetSystemLibrary.IsValid` _array_element)
        (bind (_islighted _lightaxis _lightpos _lightangle _lightradius) (`self.Get Light Info at Bone Pos` _returnvalue_7 _array_element))
        (if _islighted
          (bind _returnvalue_11 (`KismetMaterialLibrary.GetScalarParameterValue` "/Game/GeneralMaterials/Lights/Boy_Sockets.Boy_Sockets" "HandR_Light"))
          (if (<= _returnvalue_11 0.0)
            (`/Engine/EditorBlueprintResources/StandardMacros.IncrementInt` (`local.NLightedBones`)
              (:`  `
                (`KismetMaterialLibrary.SetScalarParameterValue` "/Game/GeneralMaterials/Lights/Boy_Sockets.Boy_Sockets" "HandR_Light" 1.0 :!label _label)
                (`KismetMaterialLibrary.SetScalarParameterValue` "/Game/GeneralMaterials/Lights/Boy_Sockets.Boy_Sockets" "HandR_LightRadius" _lightradius)
                (`KismetMaterialLibrary.SetScalarParameterValue` "/Game/GeneralMaterials/Lights/Boy_Sockets.Boy_Sockets" "HandR_LightAngle" _lightangle)
                (`KismetMaterialLibrary.SetVectorParameterValue` "/Game/GeneralMaterials/Lights/Boy_Sockets.Boy_Sockets" "HandR_LightAxis" (`KismetMathLibrary.Conv_VectorToLinearColor` _lightaxis))
                (`KismetMaterialLibrary.SetVectorParameterValue` "/Game/GeneralMaterials/Lights/Boy_Sockets.Boy_Sockets" "HandR_LightPos" (`KismetMathLibrary.Conv_VectorToLinearColor` _lightpos))))
            (else
              (bind _returnvalue_12 (`KismetMaterialLibrary.GetVectorParameterValue` "/Game/GeneralMaterials/Lights/Boy_Sockets.Boy_Sockets" "HandR_LightPos"))
              (if (>= (`KismetMathLibrary.Vector_Distance` _returnvalue_7 (`KismetMathLibrary.Conv_LinearColorToVector` _returnvalue_12)) (`KismetMathLibrary.Vector_Distance` _lightpos _returnvalue_7))
                (goto _label)
                (else
                  _)))))
        (bind (_islighted_2 _lightaxis_2 _lightpos_2 _lightangle_2 _lightradius_2) (`self.Get Light Info at Bone Pos` _returnvalue_8 _array_element))
        (if _islighted_2
          (bind _returnvalue_13 (`KismetMaterialLibrary.GetScalarParameterValue` "/Game/GeneralMaterials/Lights/Boy_Sockets.Boy_Sockets" "HandL_Light"))
          (if (<= _returnvalue_13 0.0)
            (`/Engine/EditorBlueprintResources/StandardMacros.IncrementInt` (`local.NLightedBones`)
              (:`  `
                (`KismetMaterialLibrary.SetScalarParameterValue` "/Game/GeneralMaterials/Lights/Boy_Sockets.Boy_Sockets" "HandL_Light" 1.0 :!label _label_2)
                (`KismetMaterialLibrary.SetScalarParameterValue` "/Game/GeneralMaterials/Lights/Boy_Sockets.Boy_Sockets" "HandL_LightAngle" _lightangle_2)
                (`KismetMaterialLibrary.SetScalarParameterValue` "/Game/GeneralMaterials/Lights/Boy_Sockets.Boy_Sockets" "HandL_LightRadius" _lightradius_2)
                (`KismetMaterialLibrary.SetVectorParameterValue` "/Game/GeneralMaterials/Lights/Boy_Sockets.Boy_Sockets" "HandL_LightAxis" (`KismetMathLibrary.Conv_VectorToLinearColor` _lightaxis_2))
                (`KismetMaterialLibrary.SetVectorParameterValue` "/Game/GeneralMaterials/Lights/Boy_Sockets.Boy_Sockets" "HandL_LightPos" (`KismetMathLibrary.Conv_VectorToLinearColor` _lightpos_2))))
            (else
              (bind _returnvalue_14 (`KismetMaterialLibrary.GetVectorParameterValue` "/Game/GeneralMaterials/Lights/Boy_Sockets.Boy_Sockets" "HandL_LightPos"))
              (if (>= (`KismetMathLibrary.Vector_Distance` _returnvalue_8 (`KismetMathLibrary.Conv_LinearColorToVector` _returnvalue_14)) (`KismetMathLibrary.Vector_Distance` _lightpos_2 _returnvalue_8))
                (goto _label_2)
                (else
                  _)))))
        (bind (_islighted_3 _lightaxis_3 _lightpos_3 _lightangle_3 _lightradius_3) (`self.Get Light Info at Bone Pos` _returnvalue_5 _array_element))
        (if _islighted_3
          (bind _returnvalue_15 (`KismetMaterialLibrary.GetScalarParameterValue` "/Game/GeneralMaterials/Lights/Boy_Sockets.Boy_Sockets" "ArmR_Light"))
          (if (<= _returnvalue_15 0.0)
            (`/Engine/EditorBlueprintResources/StandardMacros.IncrementInt` (`local.NLightedBones`)
              (:`  `
                (`KismetMaterialLibrary.SetScalarParameterValue` "/Game/GeneralMaterials/Lights/Boy_Sockets.Boy_Sockets" "ArmR_Light" 1.0 :!label _label_3)
                (`KismetMaterialLibrary.SetScalarParameterValue` "/Game/GeneralMaterials/Lights/Boy_Sockets.Boy_Sockets" "ArmR_LightAngle" _lightangle_3)
                (`KismetMaterialLibrary.SetScalarParameterValue` "/Game/GeneralMaterials/Lights/Boy_Sockets.Boy_Sockets" "ArmR_LightRadius" _lightradius_3)
                (`KismetMaterialLibrary.SetVectorParameterValue` "/Game/GeneralMaterials/Lights/Boy_Sockets.Boy_Sockets" "ArmR_LightAxis" (`KismetMathLibrary.Conv_VectorToLinearColor` _lightaxis_3))
                (`KismetMaterialLibrary.SetVectorParameterValue` "/Game/GeneralMaterials/Lights/Boy_Sockets.Boy_Sockets" "ArmR_LightPos" (`KismetMathLibrary.Conv_VectorToLinearColor` _lightpos_3))))
            (else
              (bind _returnvalue_16 (`KismetMaterialLibrary.GetVectorParameterValue` "/Game/GeneralMaterials/Lights/Boy_Sockets.Boy_Sockets" "ArmR_LightPos"))
              (if (>= (`KismetMathLibrary.Vector_Distance` _returnvalue_5 (`KismetMathLibrary.Conv_LinearColorToVector` _returnvalue_16)) (`KismetMathLibrary.Vector_Distance` _lightpos_3 _returnvalue_5))
                (goto _label_3)
                (else
                  _)))))
        (bind (_islighted_4 _lightaxis_4 _lightpos_4 _lightangle_4 _lightradius_4) (`self.Get Light Info at Bone Pos` _returnvalue _array_element))
        (if _islighted_4
          (bind _returnvalue_17 (`KismetMaterialLibrary.GetScalarParameterValue` "/Game/GeneralMaterials/Lights/Boy_Sockets.Boy_Sockets" "ArmL_Light"))
          (if (<= _returnvalue_17 0.0)
            (`/Engine/EditorBlueprintResources/StandardMacros.IncrementInt` (`local.NLightedBones`)
              (:`  `
                (`KismetMaterialLibrary.SetScalarParameterValue` "/Game/GeneralMaterials/Lights/Boy_Sockets.Boy_Sockets" "ArmL_Light" 1.0 :!label _label_4)
                (`KismetMaterialLibrary.SetScalarParameterValue` "/Game/GeneralMaterials/Lights/Boy_Sockets.Boy_Sockets" "ArmL_LightAngle" _lightangle_4)
                (`KismetMaterialLibrary.SetScalarParameterValue` "/Game/GeneralMaterials/Lights/Boy_Sockets.Boy_Sockets" "ArmL_LightRadius" _lightradius_4)
                (`KismetMaterialLibrary.SetVectorParameterValue` "/Game/GeneralMaterials/Lights/Boy_Sockets.Boy_Sockets" "ArmL_LightAxis" (`KismetMathLibrary.Conv_VectorToLinearColor` _lightaxis_4))
                (`KismetMaterialLibrary.SetVectorParameterValue` "/Game/GeneralMaterials/Lights/Boy_Sockets.Boy_Sockets" "ArmL_LightPos" (`KismetMathLibrary.Conv_VectorToLinearColor` _lightpos_4))))
            (else
              (bind _returnvalue_18 (`KismetMaterialLibrary.GetVectorParameterValue` "/Game/GeneralMaterials/Lights/Boy_Sockets.Boy_Sockets" "ArmL_LightPos"))
              (if (>= (`KismetMathLibrary.Vector_Distance` _returnvalue (`KismetMathLibrary.Conv_LinearColorToVector` _returnvalue_18)) (`KismetMathLibrary.Vector_Distance` _lightpos_4 _returnvalue))
                (goto _label_4)
                (else
                  _)))))
        (bind (_islighted_5 _lightaxis_5 _lightpos_5 _lightangle_5 _lightradius_5) (`self.Get Light Info at Bone Pos` _returnvalue_6 _array_element))
        (if _islighted_5
          (bind _returnvalue_19 (`KismetMaterialLibrary.GetScalarParameterValue` "/Game/GeneralMaterials/Lights/Boy_Sockets.Boy_Sockets" "Torso_Light"))
          (if (<= _returnvalue_19 0.0)
            (`/Engine/EditorBlueprintResources/StandardMacros.IncrementInt` (`local.NLightedBones`)
              (:`  `
                (`KismetMaterialLibrary.SetScalarParameterValue` "/Game/GeneralMaterials/Lights/Boy_Sockets.Boy_Sockets" "Torso_Light" 1.0 :!label _label_5)
                (`KismetMaterialLibrary.SetScalarParameterValue` "/Game/GeneralMaterials/Lights/Boy_Sockets.Boy_Sockets" "Torso_LightAngle" _lightangle_5)
                (`KismetMaterialLibrary.SetScalarParameterValue` "/Game/GeneralMaterials/Lights/Boy_Sockets.Boy_Sockets" "Torso_LightRadius" _lightradius_5)
                (`KismetMaterialLibrary.SetVectorParameterValue` "/Game/GeneralMaterials/Lights/Boy_Sockets.Boy_Sockets" "Torso_LightAxis" (`KismetMathLibrary.Conv_VectorToLinearColor` _lightaxis_5))
                (`KismetMaterialLibrary.SetVectorParameterValue` "/Game/GeneralMaterials/Lights/Boy_Sockets.Boy_Sockets" "Torso_LightPos" (`KismetMathLibrary.Conv_VectorToLinearColor` _lightpos_5))))
            (else
              (bind _returnvalue_20 (`KismetMaterialLibrary.GetVectorParameterValue` "/Game/GeneralMaterials/Lights/Boy_Sockets.Boy_Sockets" "Torso_LightPos"))
              (if (>= (`KismetMathLibrary.Vector_Distance` _returnvalue_6 (`KismetMathLibrary.Conv_LinearColorToVector` _returnvalue_20)) (`KismetMathLibrary.Vector_Distance` _lightpos_5 _returnvalue_6))
                (goto _label_5)
                (else
                  _)))))
        (bind (_islighted_6 _lightaxis_6 _lightpos_6 _lightangle_6 _lightradius_6) (`self.Get Light Info at Bone Pos` _returnvalue_2 _array_element))
        (if _islighted_6
          (bind _returnvalue_21 (`KismetMaterialLibrary.GetScalarParameterValue` "/Game/GeneralMaterials/Lights/Boy_Sockets.Boy_Sockets" "Head_Light"))
          (if (<= _returnvalue_21 0.0)
            (`/Engine/EditorBlueprintResources/StandardMacros.IncrementInt` (`local.NLightedBones`)
              (:`  `
                (`KismetMaterialLibrary.SetScalarParameterValue` "/Game/GeneralMaterials/Lights/Boy_Sockets.Boy_Sockets" "Head_Light" 1.0 :!label _label_6)
                (`KismetMaterialLibrary.SetScalarParameterValue` "/Game/GeneralMaterials/Lights/Boy_Sockets.Boy_Sockets" "Head_LightAngle" _lightangle_6)
                (`KismetMaterialLibrary.SetScalarParameterValue` "/Game/GeneralMaterials/Lights/Boy_Sockets.Boy_Sockets" "Head_LightRadius" _lightradius_6)
                (`KismetMaterialLibrary.SetVectorParameterValue` "/Game/GeneralMaterials/Lights/Boy_Sockets.Boy_Sockets" "Head_LightAxis" (`KismetMathLibrary.Conv_VectorToLinearColor` _lightaxis_6))
                (`KismetMaterialLibrary.SetVectorParameterValue` "/Game/GeneralMaterials/Lights/Boy_Sockets.Boy_Sockets" "Head_LightPos" (`KismetMathLibrary.Conv_VectorToLinearColor` _lightpos_6))))
            (else
              (bind _returnvalue_22 (`KismetMaterialLibrary.GetVectorParameterValue` "/Game/GeneralMaterials/Lights/Boy_Sockets.Boy_Sockets" "Head_LightPos"))
              (if (>= (`KismetMathLibrary.Vector_Distance` _returnvalue_2 (`KismetMathLibrary.Conv_LinearColorToVector` _returnvalue_22)) (`KismetMathLibrary.Vector_Distance` _lightpos_6 _returnvalue_2))
                (goto _label_6)
                (else
                  _)))))
        (bind (_islighted_7 _lightaxis_7 _lightpos_7 _lightangle_7 _lightradius_7) (`self.Get Light Info at Bone Pos` _returnvalue_9 _array_element))
        (if _islighted_7
          (bind _returnvalue_23 (`KismetMaterialLibrary.GetScalarParameterValue` "/Game/GeneralMaterials/Lights/Boy_Sockets.Boy_Sockets" "LegR_Light"))
          (if (<= _returnvalue_23 0.0)
            (`/Engine/EditorBlueprintResources/StandardMacros.IncrementInt` (`local.NLightedBones`)
              (:`  `
                (`KismetMaterialLibrary.SetScalarParameterValue` "/Game/GeneralMaterials/Lights/Boy_Sockets.Boy_Sockets" "LegR_Light" 1.0 :!label _label_7)
                (`KismetMaterialLibrary.SetScalarParameterValue` "/Game/GeneralMaterials/Lights/Boy_Sockets.Boy_Sockets" "LegR_LightAngle" _lightangle_7)
                (`KismetMaterialLibrary.SetScalarParameterValue` "/Game/GeneralMaterials/Lights/Boy_Sockets.Boy_Sockets" "LegR_LightRadius" _lightradius_7)
                (`KismetMaterialLibrary.SetVectorParameterValue` "/Game/GeneralMaterials/Lights/Boy_Sockets.Boy_Sockets" "LegR_LightAxis" (`KismetMathLibrary.Conv_VectorToLinearColor` _lightaxis_7))
                (`KismetMaterialLibrary.SetVectorParameterValue` "/Game/GeneralMaterials/Lights/Boy_Sockets.Boy_Sockets" "LegR_LightPos" (`KismetMathLibrary.Conv_VectorToLinearColor` _lightpos_7))))
            (else
              (bind _returnvalue_24 (`KismetMaterialLibrary.GetVectorParameterValue` "/Game/GeneralMaterials/Lights/Boy_Sockets.Boy_Sockets" "LegR_LightPos"))
              (if (>= (`KismetMathLibrary.Vector_Distance` _returnvalue_9 (`KismetMathLibrary.Conv_LinearColorToVector` _returnvalue_24)) (`KismetMathLibrary.Vector_Distance` _lightpos_7 _returnvalue_9))
                (goto _label_7)
                (else
                  _)))))
        (bind (_islighted_8 _lightaxis_8 _lightpos_8 _lightangle_8 _lightradius_8) (`self.Get Light Info at Bone Pos` _returnvalue_10 _array_element))
        (if _islighted_8
          (bind _returnvalue_25 (`KismetMaterialLibrary.GetScalarParameterValue` "/Game/GeneralMaterials/Lights/Boy_Sockets.Boy_Sockets" "LegL_Light"))
          (if (<= _returnvalue_25 0.0)
            (`/Engine/EditorBlueprintResources/StandardMacros.IncrementInt` (`local.NLightedBones`)
              (:`  `
                (`KismetMaterialLibrary.SetScalarParameterValue` "/Game/GeneralMaterials/Lights/Boy_Sockets.Boy_Sockets" "LegL_Light" 1.0 :!label _label_8)
                (`KismetMaterialLibrary.SetScalarParameterValue` "/Game/GeneralMaterials/Lights/Boy_Sockets.Boy_Sockets" "LegL_LightAngle" _lightangle_8)
                (`KismetMaterialLibrary.SetScalarParameterValue` "/Game/GeneralMaterials/Lights/Boy_Sockets.Boy_Sockets" "LegL_LightRadius" _lightradius_8)
                (`KismetMaterialLibrary.SetVectorParameterValue` "/Game/GeneralMaterials/Lights/Boy_Sockets.Boy_Sockets" "LegL_LightAxis" (`KismetMathLibrary.Conv_VectorToLinearColor` _lightaxis_8))
                (`KismetMaterialLibrary.SetVectorParameterValue` "/Game/GeneralMaterials/Lights/Boy_Sockets.Boy_Sockets" "LegL_LightPos" (`KismetMathLibrary.Conv_VectorToLinearColor` _lightpos_8))))
            (else
              (bind _returnvalue_26 (`KismetMaterialLibrary.GetVectorParameterValue` "/Game/GeneralMaterials/Lights/Boy_Sockets.Boy_Sockets" "LegL_LightPos"))
              (if (>= (`KismetMathLibrary.Vector_Distance` _returnvalue_10 (`KismetMathLibrary.Conv_LinearColorToVector` _returnvalue_26)) (`KismetMathLibrary.Vector_Distance` _lightpos_8 _returnvalue_10))
                (goto _label_8)
                (else
                  _)))))
        (bind (_islighted_9 _lightaxis_9 _lightpos_9 _lightangle_9 _lightradius_9) (`self.Get Light Info at Bone Pos` _returnvalue_3 _array_element))
        (if _islighted_9
          (bind _returnvalue_27 (`KismetMaterialLibrary.GetScalarParameterValue` "/Game/GeneralMaterials/Lights/Boy_Sockets.Boy_Sockets" "FootR_Light"))
          (if (<= _returnvalue_27 0.0)
            (`/Engine/EditorBlueprintResources/StandardMacros.IncrementInt` (`local.NLightedBones`)
              (:`  `
                (`KismetMaterialLibrary.SetScalarParameterValue` "/Game/GeneralMaterials/Lights/Boy_Sockets.Boy_Sockets" "FootR_Light" 1.0 :!label _label_9)
                (`KismetMaterialLibrary.SetScalarParameterValue` "/Game/GeneralMaterials/Lights/Boy_Sockets.Boy_Sockets" "FootR_LightAngle" _lightangle_9)
                (`KismetMaterialLibrary.SetScalarParameterValue` "/Game/GeneralMaterials/Lights/Boy_Sockets.Boy_Sockets" "FootR_LightRadius" _lightradius_9)
                (`KismetMaterialLibrary.SetVectorParameterValue` "/Game/GeneralMaterials/Lights/Boy_Sockets.Boy_Sockets" "FootR_LightAxis" (`KismetMathLibrary.Conv_VectorToLinearColor` _lightaxis_9))
                (`KismetMaterialLibrary.SetVectorParameterValue` "/Game/GeneralMaterials/Lights/Boy_Sockets.Boy_Sockets" "FootR_LightPos" (`KismetMathLibrary.Conv_VectorToLinearColor` _lightpos_9))))
            (else
              (bind _returnvalue_28 (`KismetMaterialLibrary.GetVectorParameterValue` "/Game/GeneralMaterials/Lights/Boy_Sockets.Boy_Sockets" "FootR_LightPos"))
              (if (>= (`KismetMathLibrary.Vector_Distance` _returnvalue_3 (`KismetMathLibrary.Conv_LinearColorToVector` _returnvalue_28)) (`KismetMathLibrary.Vector_Distance` _lightpos_9 _returnvalue_3))
                (goto _label_9)
                (else
                  _)))))
        (bind (_islighted_10 _lightaxis_10 _lightpos_10 _lightangle_10 _lightradius_10) (`self.Get Light Info at Bone Pos` _returnvalue_4 _array_element))
        (if _islighted_10
          (bind _returnvalue_29 (`KismetMaterialLibrary.GetScalarParameterValue` "/Game/GeneralMaterials/Lights/Boy_Sockets.Boy_Sockets" "FootL_Light"))
          (if (<= _returnvalue_29 0.0)
            (`/Engine/EditorBlueprintResources/StandardMacros.IncrementInt` (`local.NLightedBones`)
              (:`  `
                (`KismetMaterialLibrary.SetScalarParameterValue` "/Game/GeneralMaterials/Lights/Boy_Sockets.Boy_Sockets" "FootL_Light" 1.0 :!label _label_10)
                (`KismetMaterialLibrary.SetScalarParameterValue` "/Game/GeneralMaterials/Lights/Boy_Sockets.Boy_Sockets" "FootL_LightAngle" _lightangle_10)
                (`KismetMaterialLibrary.SetScalarParameterValue` "/Game/GeneralMaterials/Lights/Boy_Sockets.Boy_Sockets" "FootL_LightRadius" _lightradius_10)
                (`KismetMaterialLibrary.SetVectorParameterValue` "/Game/GeneralMaterials/Lights/Boy_Sockets.Boy_Sockets" "FootL_LightAxis" (`KismetMathLibrary.Conv_VectorToLinearColor` _lightaxis_10))
                (`KismetMaterialLibrary.SetVectorParameterValue` "/Game/GeneralMaterials/Lights/Boy_Sockets.Boy_Sockets" "FootL_LightPos" (`KismetMathLibrary.Conv_VectorToLinearColor` _lightpos_10))))
            (else
              (bind _returnvalue_30 (`KismetMaterialLibrary.GetVectorParameterValue` "/Game/GeneralMaterials/Lights/Boy_Sockets.Boy_Sockets" "FootL_LightPos"))
              (if (>= (`KismetMathLibrary.Vector_Distance` _returnvalue_4 (`KismetMathLibrary.Conv_LinearColorToVector` _returnvalue_30)) (`KismetMathLibrary.Vector_Distance` _lightpos_10 _returnvalue_4))
                (goto _label_10))))))))
  ;[1 1 1] Set heart variables
  (set `local.HeartPos` (`SceneComponent.GetSocketLocation` (`self.Mesh`) "Heart"))
  (if (`KismetArrayLibrary.Array_IsEmpty` _lights)
    (set `local.IsHeartLighted` false)
    (set `local.HeartAlpha` 1.0)
    (else
      (for _array_element_2 _lights
        (if (`KismetSystemLibrary.IsValid` _array_element_2)
          (bind _islighted_11 (`self.Get Light Info at Heart` (`local.HeartPos`) _array_element_2))
          (bind _output_get (set `local.IsHeartLighted` _islighted_11))
          (if _output_get
            (break))))
      (if (`local.IsHeartLighted`)
        (set `local.HeartAlpha` 0.0)
        (else
          (set `local.HeartAlpha` (/ (`KismetMathLibrary.Conv_IntToDouble` (- 10 (`local.NLightedBones`))) 10.0))))))
  (`FXSystemComponent.SetVectorParameter` _ns_boy "HeartPos" (`local.HeartPos`))
  (`FXSystemComponent.SetFloatParameter` _ns_boy "HeartAlpha" (`local.HeartAlpha`))
  (`FXSystemComponent.SetBoolParameter` _ns_boy "HeartLighted" _isheartlighted)
  (bind _output_get_2 (set `self.HeartIsLighted` _isheartlighted))
  (bind _output_get_3 (set `self.bIsInMaterialForm` _output_get_2))
  (if _output_get_3
    (`CapsuleComponent.SetCapsuleRadius` _capsulecomponent (`self.CapsuleRadius`) true)
    (else
      (`CapsuleComponent.SetCapsuleRadius` _capsulecomponent 5.0 true))))

(fn `UserConstructionScript`
  (if (`self.isEditor`)
    (`KismetMaterialLibrary.SetScalarParameterValue` "/Game/GeneralMaterials/Lights/Boy_Sockets.Boy_Sockets" "IsEditor" 1.0)
    (else
      (`KismetMaterialLibrary.SetScalarParameterValue` "/Game/GeneralMaterials/Lights/Boy_Sockets.Boy_Sockets" "IsEditor" -1.0))))