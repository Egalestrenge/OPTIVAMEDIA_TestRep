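; Level 3 switch behaviour that shuts down the generator and opens the big door when its bound switch triggers.
; A timeline fades spotlights, lights, boxes and wall cable emissives through dynamic material instances recreated each update, while deactivating unreachable lights and box character detection.
; When the fade finishes, it spawns Niagara door particles at hard-coded coordinates, plays the wall audio and slides both door halves apart along X.
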(event `SwitchTriggered`
  (params (LeverPosition :type "/Game/GeneralBlueprints/Switches/SwitchPositions Enum" :default "NewEnumerator0"))
  (bind _returnvalue (`KismetMathLibrary.MakeVector` 423.254941 -1245.130308))
  (bind _returnvalue_2 (`self.GetComponentByClass` (`self.Generator`) "/Script/Engine.AudioComponent"))
  (bind _staticmeshcomponent (`StaticMeshActor.StaticMeshComponent` (`self.DoorL`)))
  (bind _staticmeshcomponent_2 (`StaticMeshActor.StaticMeshComponent` (`self.DoorR`)))
  (bind (_returnvalue_x _returnvalue_y _returnvalue_z) (`KismetMathLibrary.BreakVector` (`SceneComponent.K2_GetComponentLocation` _staticmeshcomponent)))
  (bind (_returnvalue_x_2 _returnvalue_y_2 _returnvalue_z_2) (`KismetMathLibrary.BreakVector` (`SceneComponent.K2_GetComponentLocation` _staticmeshcomponent_2)))
  (`AudioComponent.Stop` _returnvalue_2)
  (`GameplayStatics.PlaySoundAtLocation` "/Game/Sounds/Files/GeneratorTurnOff.GeneratorTurnOff" (`SceneComponent.K2_GetComponentLocation` _returnvalue_2) (struct) 1.0 1.0 0.0 (`AudioComponent.AttenuationSettings` _returnvalue_2) null null null)
  (bind (_direction _intensity) (`Timeline|TurnOffLights`)
    (:`Update`
      (for _array_element (`self.Spotlights`)
        ;[1 1 1] Spotlights
        (`LightComponent.SetIntensity` (`/Game/Levels/03_CityDoor/Blueprints/BP_Spotlight.SpotLight` _array_element) _intensity)
        (bind _returnvalue_3 (`KismetMaterialLibrary.CreateDynamicMaterialInstance` "/Game/Levels/03_CityDoor/Meshes/SpotlightInterior_MAT_Inst.SpotlightInterior_MAT_Inst"))
        (`MaterialInstanceDynamic.SetScalarParameterValue` _returnvalue_3 "EmissiveIntensity" _intensity)
        (`PrimitiveComponent.SetMaterial` (`/Game/Levels/03_CityDoor/Blueprints/BP_Spotlight.SpotlightMesh` _array_element) 1 _returnvalue_3)
        (bind _asbp_unreachable_light (cast `/Game/GeneralBlueprints/BP_UnreachableLight` (`ChildActorComponent.ChildActor` (`/Game/Levels/03_CityDoor/Blueprints/BP_Spotlight.BP_Light` _array_element))))
        (set `UnreachableLight.bIsActive` false _asbp_unreachable_light)
        (`ActorComponent.ToggleActive` (`/Game/Levels/03_CityDoor/Blueprints/BP_Spotlight.HangingParticules_System` _array_element)))
      (for _array_element_2 (`self.Lights`)
        ;[1 1 1] Lights
        (`LightComponent.SetIntensity` (`Light.LightComponent` _array_element_2) _intensity))
      (for _array_element_3 (`self.Boxes`)
        ;[1 1 1] Boxes
        (bind _returnvalue_4 (`KismetMaterialLibrary.CreateDynamicMaterialInstance` "/Game/Levels/03_CityDoor/Meshes/BoxTopFlex_MAT_Inst.BoxTopFlex_MAT_Inst"))
        (`MaterialInstanceDynamic.SetScalarParameterValue` _returnvalue_4 "EmissiveIntensity" _intensity)
        (`PrimitiveComponent.SetMaterial` (`/Game/Levels/03_CityDoor/Blueprints/BP_ControlBox.TopFlex` _array_element_3) 0 _returnvalue_4)
        (`PrimitiveComponent.SetMaterial` (`/Game/Levels/03_CityDoor/Blueprints/BP_ControlBox.TopFlex2` _array_element_3) 0 _returnvalue_4)
        (`PrimitiveComponent.SetMaterial` (`/Game/Levels/03_CityDoor/Blueprints/BP_ControlBox.TopFlex3` _array_element_3) 0 _returnvalue_4)
        (`PrimitiveComponent.SetMaterial` (`/Game/Levels/03_CityDoor/Blueprints/BP_ControlBox.TopFlex4` _array_element_3) 0 _returnvalue_4)
        (bind _returnvalue_5 (`KismetMaterialLibrary.CreateDynamicMaterialInstance` "/Game/Levels/03_CityDoor/Meshes/ControlBoxWindowGlass_MAT_Inst.ControlBoxWindowGlass_MAT_Inst"))
        (`MaterialInstanceDynamic.SetScalarParameterValue` _returnvalue_5 "EmissiveIntensity" _intensity)
        (bind _controlbox (`/Game/Levels/03_CityDoor/Blueprints/BP_ControlBox.ControlBox` _array_element_3))
        (`PrimitiveComponent.SetMaterialByName` _controlbox "ControlBoxWindowGlass_MAT" _returnvalue_5)
        (bind _returnvalue_6 (`KismetMaterialLibrary.CreateDynamicMaterialInstance` "/Game/Levels/03_CityDoor/Meshes/BoxControlFlex_MAT_Inst.BoxControlFlex_MAT_Inst"))
        (`MaterialInstanceDynamic.SetScalarParameterValue` _returnvalue_6 "EmissiveIntensity" _intensity)
        (`PrimitiveComponent.SetMaterialByName` _controlbox "ControlBoxFlex_MAT" _returnvalue_6)
        (set `/Game/Levels/03_CityDoor/Blueprints/BP_ControlBox.CanDetectCharacter` false _array_element_3))
      (bind _returnvalue_7 (`KismetMaterialLibrary.CreateDynamicMaterialInstance` "/Game/Levels/03_CityDoor/Meshes/CableWall_MAT_Inst.CableWall_MAT_Inst"))
      ;[1 1 1] BigWall
      (`MaterialInstanceDynamic.SetScalarParameterValue` _returnvalue_7 "EmissiveIntensity" _intensity)
      (`MaterialInstanceDynamic.SetVectorParameterValue` :`self` _returnvalue_7 :`ParameterName` "BaseColor")
      (`PrimitiveComponent.SetMaterial` (`StaticMeshActor.StaticMeshComponent` (`self.BigWall`)) 2 _returnvalue_7)
      ;[1 1 1] Unreachable lights
      (for _array_element_4 (`self.UnreachableLights`)
        (set `UnreachableLight.bIsActive` false _array_element_4)))
    (:`Finished`
      ;[1 1 1] OpenDoor event
      (bind _returnvalue_8 (`NiagaraFunctionLibrary.SpawnSystemAttached` "/Game/GeneralProps/Doors/Particles/NS_DoorParticles.NS_DoorParticles" (`self.DefaultSceneRoot`) "None" _returnvalue (struct :`Yaw` 90.0) "KeepWorldPosition" true))
      (`FXSystemComponent.SetFloatParameter` _returnvalue_8 "DoorH" (`KismetMathLibrary.Vector_Distance` _returnvalue (`KismetMathLibrary.MakeVector` 423.254941 -1245.130308 770.0)))
      (`FXSystemComponent.SetFloatParameter` _returnvalue_8 "DoorW" 10.0)
      (set `self.DoorLXLocation` _returnvalue_x)
      (set `self.DoorRXLocation` _returnvalue_x_2)
      (`AudioComponent.Play` (`self.GetComponentByClass` (`self.BigWall`) "/Script/Engine.AudioComponent") 0.0)
      (bind (_direction_2 _doorxtranslation) (`Timeline|OpenDoor`)
        (:`Update`
          (`SceneComponent.K2_SetWorldLocation` _staticmeshcomponent (`KismetMathLibrary.MakeVector` (+ (`self.DoorLXLocation`) (* _doorxtranslation -1.0)) _returnvalue_y _returnvalue_z) false false)
          (`SceneComponent.K2_SetWorldLocation` _staticmeshcomponent_2 (`KismetMathLibrary.MakeVector` (+ (`self.DoorRXLocation`) _doorxtranslation) _returnvalue_y_2 _returnvalue_z_2) false false))))))

(event `self.ReceiveBeginPlay`
  (add `/Game/GeneralBlueprints/Switches/BP_Switch.SwitchTriggered` (`self.Switch`) (delegate `SwitchTriggered`)))

(fn `UserConstructionScript`
  (`parent.UserConstructionScript`))