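; BP_Switch is an interactable lever switch whose handle visually follows a bone on the character operating it.
; Lever start movement begins a looping frame-time timer that runs MoveLever, deriving roll from the bone's lever-local position via arctangent and smoothing it with FInterpTo.
; End movement stops the timer, toggles the Up/Down state, disables the child interact region and calls SwitchTriggered with the new state.
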(event `self.ReceiveBeginPlay`
  (add `self.LeverStartMovement` (delegate `StartLeverMovement`))
  (add `self.LeverEndMovement` (delegate `EndLeverMovement`)))

(event `StartLeverMovement` :!signature `self.LeverStartMovement`
  (params (Character :type "/Game/Characters/General/BP_GeneralCharacter Object Reference") (BoneToTrack :type Name))
  (bind _returnvalue (`KismetSystemLibrary.K2_SetTimerDelegate` (delegate `StartMovement`) (`GameplayStatics.GetWorldDeltaSeconds`) true))
  (set `self.LeverTimer` _returnvalue))

(event `StartMovement`
  (`self.MoveLever` (stale `StartLeverMovement` Character) (stale `StartLeverMovement` BoneToTrack)))

(event `EndLeverMovement`
  (`KismetSystemLibrary.K2_ClearAndInvalidateTimerHandle` (`self.LeverTimer`))
  (switch `/Game/GeneralBlueprints/Switches/SwitchPositions` (`self.LeverPos`)
    (:`NewEnumerator0`
      (set `self.LeverPos` "NewEnumerator1"))
    (:`NewEnumerator1`
      (set `self.LeverPos` "NewEnumerator0")))
  (bind _asbp_interact_region (cast `/Game/GeneralBlueprints/BP_InteractRegion` (`ChildActorComponent.ChildActor` (`self.InteractionRegion`))))
  (set `/Game/GeneralBlueprints/BP_InteractRegion.CanInteract` false _asbp_interact_region)
  (`self.SwitchTriggered` (`self.LeverPos`)))

(fn `MoveLever`
  (params (Character :type "/Game/Characters/General/BP_GeneralCharacter Object Reference") (BoneToTrack :type Name))
  (bind _lever (`self.Lever`))
  (bind _relativerotation_roll (`KismetMathLibrary.BreakRotator` (`SceneComponent.RelativeRotation` _lever)))
  (bind (_returnvalue_x _returnvalue_y _returnvalue_z) (`KismetMathLibrary.BreakVector` (`KismetMathLibrary.InverseTransformLocation` (`SceneComponent.K2_GetComponentToWorld` (`self.Lever`)) (`SceneComponent.GetSocketLocation` (`Character.Mesh` Character) BoneToTrack))))
  (`SceneComponent.K2_SetRelativeRotation` _lever (`KismetMathLibrary.MakeRotator` (`KismetMathLibrary.FInterpTo` _relativerotation_roll (- _relativerotation_roll (`KismetMathLibrary.DegAtan` (/ _returnvalue_z _returnvalue_y))) (`GameplayStatics.GetWorldDeltaSeconds`) 10.0)) false false))

(fn `UserConstructionScript`)