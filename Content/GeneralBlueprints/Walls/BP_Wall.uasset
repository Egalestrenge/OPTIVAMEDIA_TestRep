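; BP_Wall is a wall actor whose only logic is a test for whether the character is facing it.
; IsTheCharacterLookingAtMe finds the point on NextEdge's spline closest to the character and compares the flattened direction to it with the character's forward vector.
; A 2D dot product of at least 0.7, roughly a 45-degree cone either side, counts as looking.
; The event graph holds only disabled stubs.
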(fn `IsTheCharacterLookingAtMe`
  (returns (IsTheCharacterLookingAtMe :type Boolean))
  (bind _character (`self.Character`))
  (bind _returnvalue (`self.K2_GetActorLocation` _character))
  (return (>= (`KismetMathLibrary.DotProduct2D` (`KismetMathLibrary.Normal2D` (`KismetMathLibrary.Conv_VectorToVector2D` (- (`SplineComponent.FindLocationClosestToWorldLocation` (`/Game/GeneralBlueprints/Walls/BP_Edge.EdgeSpline` (`self.NextEdge`)) _returnvalue "World") _returnvalue))) (`KismetMathLibrary.Normal2D` (`KismetMathLibrary.Conv_VectorToVector2D` (`self.GetActorForwardVector` _character)))) 0.7)))

(fn `UserConstructionScript`
  (`parent.UserConstructionScript`))