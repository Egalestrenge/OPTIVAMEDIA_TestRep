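; BP_Edge is a spline-based wall edge actor that answers proximity and facing queries about a character.
; IsTheCharacterLookingAtMe compares the character's horizontal forward vector with the direction to the closest EdgeSpline point, using a dot-product threshold.
; GetDistanceToCharacter finds the spline point closest to a spot ahead of the character, but measures from the character's world location to that point in local space.
; The event graph holds no custom logic.
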(event `self.ReceiveActorBeginOverlap`
  (params (OtherActor :type "Actor Object Reference"))
  (`parent.ReceiveActorBeginOverlap` OtherActor))

(fn `GetDistanceToCharacter`
  (params (Character :type "/Game/Characters/General/BP_GeneralCharacter Object Reference"))
  (returns (Distance :type "Float (double-precision)"))
  (return (`KismetMathLibrary.Vector_Distance` (`self.K2_GetActorLocation` Character) (`SplineComponent.FindLocationClosestToWorldLocation` (`self.EdgeSpline`) (`KismetMathLibrary.TransformLocation` (`self.GetTransform` Character) (100.0 0.0 0.0)) "Local"))))

(fn `IsTheCharacterLookingAtMe`
  (returns (IsTheCharacterLookingAtMe :type Boolean))
  (bind _character (`self.Character`))
  (bind _returnvalue (`self.K2_GetActorLocation` _character))
  (return (>= (`KismetMathLibrary.DotProduct2D` (`KismetMathLibrary.Normal2D` (`KismetMathLibrary.Conv_VectorToVector2D` (- (`SplineComponent.FindLocationClosestToWorldLocation` (`self.EdgeSpline`) _returnvalue "World") _returnvalue))) (`KismetMathLibrary.Normal2D` (`KismetMathLibrary.Conv_VectorToVector2D` (`self.GetActorForwardVector` _character)))) 0.7)))

(fn `UserConstructionScript`
  (`parent.UserConstructionScript`))