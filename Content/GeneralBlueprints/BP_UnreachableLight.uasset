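; Light actor that tracks characters inside its trigger by registering itself in their Lights lists.
; Overlaps update the list and signal enter or leave, while a delayed BeginPlay check catches an already overlapping BP_Boy.
; Trigger scale derives from light distance and angle plus a margin, set on construction or from width and distance.
; SetActivity plays or reverses a timeline that grows or shrinks the radius.
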(event `self.ReceiveBeginPlay`
  (bind _overlappingactors (`PrimitiveComponent.GetOverlappingActors` (`self.LightTrigger`) "/Game/Characters/Boy/Blueprints/BP_Boy.BP_Boy_C"))
  ;[1 1 1] Check for overlaping characters on begin play, and add the light to their "Lights" list
  (`KismetSystemLibrary.Delay` 0.5)
  (if (> (`KismetArrayLibrary.Array_Length` _overlappingactors) 0)
    (for _array_element _overlappingactors
      (bind _asgeneral_character (cast `GeneralCharacter` _array_element))
      (`KismetArrayLibrary.Array_Add` (`GeneralCharacter.Lights` _asgeneral_character) self))))

(event `self.LightTrigger.OnComponentBeginOverlap`
  (params (OverlappedComponent :type "PrimitiveComponent Object Reference") (OtherActor :type "Actor Object Reference") (OtherComp :type "PrimitiveComponent Object Reference") (OtherBodyIndex :type Integer) (bFromSweep :type Boolean) (SweepResult :type "HitResult Structure (by ref)"))
  ;[1 1 1] add or remove this light from the overlaping character on begin/end overlap
  (bind _asgeneral_character (cast `GeneralCharacter` OtherActor))
  (`KismetArrayLibrary.Array_Add` (`GeneralCharacter.Lights` _asgeneral_character) self)
  (`self.CharacterEnterLight` _asgeneral_character))

(event `self.LightTrigger.OnComponentEndOverlap`
  (params (OverlappedComponent :type "PrimitiveComponent Object Reference") (OtherActor :type "Actor Object Reference") (OtherComp :type "PrimitiveComponent Object Reference") (OtherBodyIndex :type Integer))
  ;[1 1 1] add or remove this light from the overlaping character on begin/end overlap
  (bind _asgeneral_character (cast `GeneralCharacter` OtherActor))
  (`KismetArrayLibrary.Array_RemoveItem` (`GeneralCharacter.Lights` _asgeneral_character) self)
  (`self.CharacterLeaveLight` _asgeneral_character))

(event `SetActivity`
  (params (IsActive :type Boolean))
  ;[1 1 1] Set light activity and change the radius
  (if IsActive
    (if (< (`self.LightRadius`) 1.0)
      (bind (_direction _radius) (`Timeline|SetRadius` :!via `PlayFromStart` :!label _label)
        (:`Update`
          (set `self.LightRadius` (* (`self.LightRadiusDefault`) _radius)))
        (:`Finished`
          (set `self.bIsActive` IsActive))))
    (elif (> (`self.LightRadius`) 1.0)
      (goto _label :!via `ReverseFromEnd`))))

(fn `AdaptTriggerSize`
  (bind _returnvalue (/ (`self.LightDistance`) 100.0))
  (bind _returnvalue_2 (* (`KismetMathLibrary.DegTan` (/ (+ (`self.LightAngle`) 30.0) 2.0)) 2.0 _returnvalue))
  (`SceneComponent.SetRelativeScale3D` (`self.LightTrigger`) (`KismetMathLibrary.MakeVector` _returnvalue _returnvalue_2 _returnvalue_2)))

(fn `SetLightSizeFromDistanceAndWidth`
  (params (Width :type "Float (double-precision)") (Distance :type "Float (double-precision)"))
  (bind _output_get (set `self.LightDistance` Distance))
  (bind _output_get_2 (set `self.LightRadius` (/ Width 2.0)))
  (set `self.LightAngle` (* (`KismetMathLibrary.DegAtan` (/ _output_get_2 _output_get)) 2.0))
  (`self.AdaptTriggerSize`))

(fn `UserConstructionScript`
  (bind _returnvalue (/ (`self.LightAngle`) 2.0))
  (`self.AdaptTriggerSize`)
  (if (`self.ShowDebugLines`)
    (`KismetSystemLibrary.DrawDebugConeInDegrees` (`self.K2_GetActorLocation`) (`self.GetActorForwardVector`) 500.0 _returnvalue _returnvalue 12 (struct :`R` 0.942708 :`G` 0.098199 :`B` 0.098199 :`A` 1.0) 0.25 1.0)))