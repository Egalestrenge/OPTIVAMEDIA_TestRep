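; BP_InteractRegion is an interaction region that provides facing and distance queries between a character and its interaction point.
; Its construction script places InteractionPoint from a configurable relative transform, and the event graph holds no active logic.
; The facing check ignores height, comparing the character's forward vector with the direction to the point through a thresholded 2D dot product.
; The distance query measures full 3D distance from character to point.
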(fn `GetDistanceToCharacter`
  (params (Character :type "/Game/Characters/General/BP_GeneralCharacter Object Reference"))
  (returns (Distance :type "Float (double-precision)"))
  (return (`KismetMathLibrary.Vector_Distance` (`self.K2_GetActorLocation` Character) (`SceneComponent.K2_GetComponentLocation` (`self.InteractionPoint`)))))

(fn `IsTheCharacterLookingAtMe`
  (returns (IsTheCharacterLookingAtMe :type Boolean))
  (bind _character (`self.Character`))
  (return (>= (`KismetMathLibrary.DotProduct2D` (`KismetMathLibrary.Normal2D` (`KismetMathLibrary.Conv_VectorToVector2D` (- (`SceneComponent.K2_GetComponentLocation` (`self.InteractionPoint`)) (`self.K2_GetActorLocation` _character)))) (`KismetMathLibrary.Normal2D` (`KismetMathLibrary.Conv_VectorToVector2D` (`self.GetActorForwardVector` _character)))) 0.7)))

(fn `UserConstructionScript`
  (`SceneComponent.K2_SetRelativeTransform` (`self.InteractionPoint`) (`self.InteractionPointTransform`) false false))