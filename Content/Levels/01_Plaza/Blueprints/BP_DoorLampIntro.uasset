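; Intro door lamp for the Plaza level that plays the boy's breathing animation when he enters its light, intended for the first entry.
; On BeginPlay it passes its ignore list to a child BP_UnreachableLight and binds to that light's enter event.
; The handler sets a "Reaching" Motion Warping target just short of the spotlight on his side, facing it.
; It then plays the breathing montage, disabling player input until completion.
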(event `PlayBreathing`
  (params (Character :type "GeneralCharacter Object Reference"))
  (bind _returnvalue (`GameplayStatics.GetPlayerController` 0))
  (bind _returnvalue_2 (`SceneComponent.K2_GetComponentLocation` (`self.SpotLight`)))
  ;[1 1 1] Play breathng animation the first time we enter this light
  (bind _asbp_boy (cast `/Game/Characters/Boy/Blueprints/BP_Boy` Character))
  (bind _returnvalue_3 (`self.K2_GetActorLocation` _asbp_boy))
  (bind (_returnvalue_x _returnvalue_y) (`KismetMathLibrary.BreakVector` (- _returnvalue_3 _returnvalue_2)))
  (bind (_returnvalue_x_2 _returnvalue_y_2) (`KismetMathLibrary.BreakVector2D` (+ (`KismetMathLibrary.Conv_VectorToVector2D` _returnvalue_2) (* (`KismetMathLibrary.Normal2D` (`KismetMathLibrary.MakeVector2D` _returnvalue_x _returnvalue_y)) (100.0 100.0)))))
  (bind (_returnvalue_roll _returnvalue_pitch _returnvalue_yaw) (`KismetMathLibrary.BreakRotator` (`KismetMathLibrary.FindLookAtRotation` _returnvalue_3 _returnvalue_2)))
  (`MotionWarpingComponent.AddOrUpdateWarpTargetFromLocationAndRotation` (`/Game/Characters/General/BP_GeneralCharacter.MotionWarping` _asbp_boy) "Reaching" (`KismetMathLibrary.MakeVector` _returnvalue_x_2 _returnvalue_y_2 10.0) (`KismetMathLibrary.MakeRotator` 0.0 0.0 _returnvalue_yaw))
  (`|PlayMontage` (`Character.Mesh` _asbp_boy) "/Game/Characters/Boy/Animations/Boy_Breathing_Montage.Boy_Breathing_Montage"
    (:`then`
      (`self.DisableInput` _asbp_boy _returnvalue))
    (:`OnCompleted`
      (`self.EnableInput` _asbp_boy _returnvalue))))

(event `self.ReceiveBeginPlay`
  (`parent.ReceiveBeginPlay`)
  (bind _asbp_unreachable_light (cast `/Game/GeneralBlueprints/BP_UnreachableLight` (`ChildActorComponent.ChildActor` (`self.BP_Light`))))
  (set `UnreachableLight.ActorsToIgnore` (`self.ActorsToIgnore`) _asbp_unreachable_light)
  (add `/Game/GeneralBlueprints/BP_UnreachableLight.CharacterEnterLight` _asbp_unreachable_light (delegate `PlayBreathing`)))

(event `self.ReceiveActorBeginOverlap`
  (params (OtherActor :type "Actor Object Reference"))
  (`parent.ReceiveActorBeginOverlap` OtherActor))

(fn `UserConstructionScript`
  (`parent.UserConstructionScript`))