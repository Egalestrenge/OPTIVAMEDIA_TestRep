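; Plaza street lamp with a spot light, emissive glass, hanging particles and a child BP_UnreachableLight.
; The construction script applies color and intensities through a dynamic material and sizes the child's trigger from cone angle and light distance.
; SetLightActive forwards only to that child.
; An Oscillate timeline can modulate glow, light and particle alpha, but nothing in this graph triggers it.
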(event `Oscillate`
  ;[1 1 1] Lamp intensity oscillation
  (bind (_direction _lightintensity _colorintensity) (`Timeline|IntensityOscillation`)
    (:`Update`
      (`MaterialInstanceDynamic.SetScalarParameterValue` (`self.Material`) "EmissiveIntensity" (* _colorintensity (`self.ColorIntensity`)))
      (`LightComponent.SetIntensity` (`self.SpotLight`) (* _lightintensity (`self.LightIntensity`)))
      (if (<= (`self.ColorIntensity`) 1.0)
        (`FXSystemComponent.SetFloatParameter` (`self.HangingParticules_System`) "ParticleAlphaMultiplier" 0.0)
        (else
          (`FXSystemComponent.SetFloatParameter` (`self.HangingParticules_System`) "ParticleAlphaMultiplier" _colorintensity))))))

(event `self.ReceiveBeginPlay`)

(event `SetLightActive`
  (params (isActive :type Boolean))
  (bind _asbp_unreachable_light (cast `/Game/GeneralBlueprints/BP_UnreachableLight` (`ChildActorComponent.ChildActor` (`self.BP_Light`))))
  (`/Game/GeneralBlueprints/BP_UnreachableLight.SetActivity` _asbp_unreachable_light isActive))

(fn `UserConstructionScript`
  (bind _material (`self.Material`))
  (bind _returnvalue (`KismetMaterialLibrary.CreateDynamicMaterialInstance` "/Game/Levels/01_Plaza/Meshes/StreetLampGlass_MAT_Inst.StreetLampGlass_MAT_Inst"))
  (bind _output_get (set `self.Material` _returnvalue))
  (`PrimitiveComponent.SetMaterial` (`self.Lamp`) 0 _output_get)
  (`MaterialInstanceDynamic.SetScalarParameterValue` _material "EmissiveIntensity" (`self.ColorIntensity`))
  (`MaterialInstanceDynamic.SetVectorParameterValue` _material "EmissiveColor" (`self.Color`))
  (`LightComponent.SetLightColor` (`self.SpotLight`) (`self.Color`) true)
  (`LightComponent.SetIntensity` (`self.SpotLight`) (`self.LightIntensity`))
  (bind _asbp_unreachable_light (cast `/Game/GeneralBlueprints/BP_UnreachableLight` (`ChildActorComponent.ChildActor` (`self.BP_Light`))))
  (set `UnreachableLight.LightAngle` (* (`SpotLightComponent.InnerConeAngle` (`self.SpotLight`)) 2.0) _asbp_unreachable_light)
  (set `UnreachableLight.LightDistance` (`self.LightDistance`) _asbp_unreachable_light)
  (`/Game/GeneralBlueprints/BP_UnreachableLight.AdaptTriggerSize` _asbp_unreachable_light)
  (if (<= (`self.ColorIntensity`) 1.0)
    (`FXSystemComponent.SetFloatParameter` (`self.HangingParticules_System`) "ParticleAlphaMultiplier" 0.0)))