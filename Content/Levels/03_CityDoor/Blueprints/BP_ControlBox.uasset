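; Control box for the CityDoor level that closes a barrier when BP_Boy enters one of three triggers while detection is enabled.
; It then listens to the boy's form-change event, reopening the barrier and unbinding once he leaves material form.
; Timelines drive the barrier's pitch, mirrored for boxes other than the BP_ControlBoxL subclass, which alone plays the barrier sound at a hardcoded location.
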(event `CloseBarrier`
  (bind _barrier (`self.Barrier`))
  (cast `/Game/Levels/03_CityDoor/Blueprints/BP_ControlBoxL` self
    (:`then`
      (`GameplayStatics.PlaySoundAtLocation` "/Game/Sounds/Files/Barrier.Barrier" (414.204254 -882.52771 58.102684) (struct) 1.0 1.0 0.0 null null null null)
      (bind (_direction _barrierangle) (`Timeline|CloseBarrierTimeline` :!via `PlayFromStart` :!label _label)
        (:`Update`
          (cast `/Game/Levels/03_CityDoor/Blueprints/BP_ControlBoxL` self
            (:`then`
              (`SceneComponent.K2_SetRelativeRotation` _barrier (`KismetMathLibrary.MakeRotator` 0.0 _barrierangle) false false))
            (:`CastFailed`
              (`SceneComponent.K2_SetRelativeRotation` _barrier (`KismetMathLibrary.MakeRotator` 0.0 (* _barrierangle -1.0)) false false))))))
    (:`CastFailed`
      (goto _label :!via `PlayFromStart`))))

(event `OpenBarrier`
  (bind _barrier (`self.Barrier`))
  (cast `/Game/Levels/03_CityDoor/Blueprints/BP_ControlBoxL` self
    (:`then`
      (`GameplayStatics.PlaySoundAtLocation` "/Game/Sounds/Files/Barrier.Barrier" (414.204254 -882.52771 58.102684) (struct) 2.0 1.0 0.0 null null null null)
      (bind (_direction _barrierangle) (`Timeline|OpenBarrierTimeline` :!via `PlayFromStart` :!label _label_2)
        (:`Update`
          (cast `/Game/Levels/03_CityDoor/Blueprints/BP_ControlBoxL` self
            (:`then`
              (`SceneComponent.K2_SetRelativeRotation` _barrier (`KismetMathLibrary.MakeRotator` 0.0 _barrierangle) false false))
            (:`CastFailed`
              (`SceneComponent.K2_SetRelativeRotation` _barrier (`KismetMathLibrary.MakeRotator` 0.0 (* _barrierangle -1.0)) false false))))))
    (:`CastFailed`
      (goto _label_2 :!via `PlayFromStart`))))

(event `self.Trigger1.OnActorBeginOverlap`
  (params (OverlappedActor :type "Actor Object Reference") (OtherActor :type "Actor Object Reference"))
  (bind _asbp_boy (cast `/Game/Characters/Boy/Blueprints/BP_Boy` OtherActor))
  (set `self.Boy` _asbp_boy)
  (if (and (`self.CanDetectCharacter`) (not (`self.Closed`))) :!label _label_3
    (add `GeneralCharacter.FFormChangedEvent` (`self.Boy`) (delegate `OpenWhenBoyDissapears`))
    (`self.CloseBarrier`)
    (set `self.Closed` true)))

(event `self.Trigger2.OnActorBeginOverlap`
  (params (OverlappedActor :type "Actor Object Reference") (OtherActor :type "Actor Object Reference"))
  (bind _asbp_boy (cast `/Game/Characters/Boy/Blueprints/BP_Boy` OtherActor))
  (set `self.Boy` _asbp_boy)
  (goto _label_3))

(event `self.Trigger3.OnActorBeginOverlap`
  (params (OverlappedActor :type "Actor Object Reference") (OtherActor :type "Actor Object Reference"))
  (bind _asbp_boy (cast `/Game/Characters/Boy/Blueprints/BP_Boy` OtherActor))
  (set `self.Boy` _asbp_boy)
  (goto _label_3))

(event `OpenWhenBoyDissapears`
  (params (bIsInMaterialForm :type Boolean))
  (if (not bIsInMaterialForm)
    (`self.OpenBarrier`)
    (set `self.Closed` false)
    (remove `GeneralCharacter.FFormChangedEvent` (`self.Boy`) (delegate `OpenWhenBoyDissapears`))))

(fn `UserConstructionScript`)