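; Floor cable in the CityDoor level that shows two lights travelling along it until its linked Switch is triggered.
; Tick loops two BP_UnreachableLight child actors along local Y up to LightEndPos, projecting their positions onto the cable axis to drive a dynamic material's glow.
; LightWidth sizes both glow and lights.
; Switching off stops movement, darkens the emissive colour and moves lights and glow positions far away.
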(event `TurnOffCable`
  (params (LeverPosition :type "/Game/GeneralBlueprints/Switches/SwitchPositions Enum" :default "NewEnumerator0"))
  (bind _returnvalue (`KismetMathLibrary.MakeColor` 0.0 2000.0 2000.0))
  (set `self.CableOn` false)
  (`MaterialInstanceDynamic.SetVectorParameterValue` (`self.Material`) "EmissiveColor" (struct :`B` 0.003 :`A` 1.0))
  (`SceneComponent.K2_SetWorldLocation` (`self.CableLight`) (0.0 2000.0 2000.0) false false)
  (`SceneComponent.K2_SetWorldLocation` (`self.CableLight2`) (0.0 1000.0 1000.0) false false)
  (`MaterialInstanceDynamic.SetVectorParameterValue` (`self.Material`) "LightPos" _returnvalue)
  (`MaterialInstanceDynamic.SetVectorParameterValue` (`self.Material`) "LightPos2" _returnvalue))

(event `self.ReceiveBeginPlay`
  (bind _lightwidth (`self.LightWidth`))
  (bind _cablelight (`self.CableLight`))
  (bind (_relativelocation_x _relativelocation_y _relativelocation_z) (`KismetMathLibrary.BreakVector` (`SceneComponent.RelativeLocation` _cablelight)))
  (add `/Game/GeneralBlueprints/Switches/BP_Switch.SwitchTriggered` (`self.Switch`) (delegate `TurnOffCable`))
  (bind _returnvalue (`KismetMaterialLibrary.CreateDynamicMaterialInstance` "/Game/Levels/03_CityDoor/Meshes/CableFloor_MAT_Inst.CableFloor_MAT_Inst"))
  (`PrimitiveComponent.SetMaterial` (`self.Cable`) 0 _returnvalue)
  (bind _output_get (set `self.Material` _returnvalue))
  (`MaterialInstanceDynamic.SetScalarParameterValue` _output_get "LightWidth" _lightwidth)
  (bind _asbp_unreachable_light (cast `/Game/GeneralBlueprints/BP_UnreachableLight` (`ChildActorComponent.ChildActor` (`self.CableLight`))))
  (bind _output_get_2 (set `/Game/GeneralBlueprints/BP_UnreachableLight.LightRadius` (/ _lightwidth 2.0) _asbp_unreachable_light))
  (bind _asbp_unreachable_light_2 (cast `/Game/GeneralBlueprints/BP_UnreachableLight` (`ChildActorComponent.ChildActor` (`self.CableLight2`))))
  (set `/Game/GeneralBlueprints/BP_UnreachableLight.LightRadius` _output_get_2 _asbp_unreachable_light_2)
  (bind _asbp_unreachable_light_3 (cast `/Game/GeneralBlueprints/BP_UnreachableLight` (`ChildActorComponent.ChildActor` _cablelight)))
  (`/Game/GeneralBlueprints/BP_UnreachableLight.SetLightSizeFromDistanceAndWidth` _asbp_unreachable_light_3 (`self.LightWidth`) _relativelocation_z))

(event `self.ReceiveTick`
  (params (DeltaSeconds :type "Float (single-precision)"))
  (bind _returnvalue (`self.GetTransform`))
  (bind _returnvalue_2 (`self.GetTransform`))
  (bind _cablelight (`self.CableLight`))
  (bind _cablelight_2 (`self.CableLight`))
  (bind _cablelight2 (`self.CableLight2`))
  (bind _cablelight2_2 (`self.CableLight2`))
  (bind (_relativelocation_x _relativelocation_y _relativelocation_z) (`KismetMathLibrary.BreakVector` (`SceneComponent.RelativeLocation` _cablelight2_2)))
  (bind (_relativelocation_x_2 _relativelocation_y_2) (`KismetMathLibrary.BreakVector` (`SceneComponent.RelativeLocation` _cablelight_2)))
  (bind (_relativelocation_x_3 _relativelocation_y_3 _relativelocation_z_2) (`KismetMathLibrary.BreakVector` (`SceneComponent.RelativeLocation` _cablelight)))
  (bind (_relativelocation_x_4 _relativelocation_y_4) (`KismetMathLibrary.BreakVector` (`SceneComponent.RelativeLocation` (`self.LightEndPos`))))
  (bind (_relativelocation_x_5 _relativelocation_y_5) (`KismetMathLibrary.BreakVector` (`SceneComponent.RelativeLocation` _cablelight2)))
  (bind (_relativelocation_x_6 _relativelocation_y_6) (`KismetMathLibrary.BreakVector` (`SceneComponent.RelativeLocation` (`self.LightEndPos`))))
  (bind (_returnvalue_x _returnvalue_y) (`KismetMathLibrary.BreakVector` (`KismetMathLibrary.InverseTransformLocation` _returnvalue_2 (`SceneComponent.K2_GetComponentLocation` (`self.CableLight2`)))))
  (bind (_returnvalue_x_2 _returnvalue_y_2) (`KismetMathLibrary.BreakVector` (`KismetMathLibrary.InverseTransformLocation` _returnvalue (`SceneComponent.K2_GetComponentLocation` (`self.CableLight`)))))
  (if (`self.CableOn`)
    (`SceneComponent.K2_AddLocalOffset` _cablelight_2 (`KismetMathLibrary.MakeVector` 0.0 (* (`self.CableLightSpeed`) (`GameplayStatics.GetWorldDeltaSeconds`))) false false)
    (if (> _relativelocation_y_2 (+ _relativelocation_y_4 (/ (`self.LightWidth`) 2.0)))
      (`SceneComponent.K2_SetRelativeLocation` _cablelight (`KismetMathLibrary.MakeVector` _relativelocation_x_3 (/ (`self.LightWidth`) -2.0) _relativelocation_z_2) false false))
    (`MaterialInstanceDynamic.SetVectorParameterValue` (`self.Material`) "LightPos" (`KismetMathLibrary.Conv_VectorToLinearColor` (`KismetMathLibrary.TransformLocation` _returnvalue (`KismetMathLibrary.MakeVector` 0.0 _returnvalue_y_2))))
    (`SceneComponent.K2_AddLocalOffset` _cablelight2 (`KismetMathLibrary.MakeVector` 0.0 (* (`self.CableLightSpeed`) (`GameplayStatics.GetWorldDeltaSeconds`))) false false)
    (if (> _relativelocation_y_5 (+ _relativelocation_y_6 (/ (`self.LightWidth`) 2.0)))
      (`SceneComponent.K2_SetRelativeLocation` _cablelight2_2 (`KismetMathLibrary.MakeVector` _relativelocation_x (/ (`self.LightWidth`) -2.0) _relativelocation_z) false false))
    (`MaterialInstanceDynamic.SetVectorParameterValue` (`self.Material`) "LightPos2" (`KismetMathLibrary.Conv_VectorToLinearColor` (`KismetMathLibrary.TransformLocation` _returnvalue_2 (`KismetMathLibrary.MakeVector` 0.0 _returnvalue_y))))))

(fn `UserConstructionScript`)