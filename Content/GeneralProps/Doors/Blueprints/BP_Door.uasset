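; Double door actor that swings open with a particle effect when its OpenDoor event is called.
; OpenDoor spawns an attached Niagara system at the bottom marker and passes it the bottom-to-top marker distance as the door height.
; A timeline then drives the yaw of both leaves, mirroring the right around 180 degrees.
; The Blueprint has no trigger or close logic of its own.
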(event `OpenDoor`
  (bind _doorparticlesspawnbottom (`self.DoorParticlesSpawnBottom`))
  ;[1 1 1] OpenDoor event
  (bind _returnvalue (`NiagaraFunctionLibrary.SpawnSystemAttached` "/Game/GeneralProps/Doors/Particles/NS_DoorParticles.NS_DoorParticles" _doorparticlesspawnbottom "None" (0.0 0.0 0.0) (struct :`Yaw` 90.0) "KeepRelativeOffset" true))
  (`FXSystemComponent.SetFloatParameter` _returnvalue "DoorH" (`KismetMathLibrary.Vector_Distance` (`SceneComponent.K2_GetComponentLocation` _doorparticlesspawnbottom) (`SceneComponent.K2_GetComponentLocation` (`self.DoorParticlesSpawnTop`))))
  (bind (_direction _doorrotation) (`Timeline|OpenDoorTimeline` :!via `PlayFromStart`)
    (:`Update`
      (`SceneComponent.K2_SetRelativeRotation` (`self.DoorL`) (`KismetMathLibrary.MakeRotator` 0.0 0.0 _doorrotation) false false)
      (`SceneComponent.K2_SetRelativeRotation` (`self.DoorR`) (`KismetMathLibrary.MakeRotator` 0.0 0.0 (- 180.0 _doorrotation)) false false))))

(fn `UserConstructionScript`)