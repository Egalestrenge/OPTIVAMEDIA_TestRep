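; AI vehicle that starts driving along a spline Path when a GeneralCharacter overlaps its Trigger.
; Each tick GetCarParams steers toward a look-ahead spline point, easing throttle and brightening brake lights on sharp turns; its Brake output is unused.
; BP_Light child actor events halt path following and brake with a sound when a character enters the light, then resume on exit.
; Engine sound pitch scales with forward speed.
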(event `self.Trigger.OnComponentBeginOverlap`
  (params (OverlappedComponent :type "PrimitiveComponent Object Reference") (OtherActor :type "Actor Object Reference") (OtherComp :type "PrimitiveComponent Object Reference") (OtherBodyIndex :type Integer) (bFromSweep :type Boolean) (SweepResult :type "HitResult Structure (by ref)"))
  (bind _vehiclemovementcomponent (`self.VehicleMovementComponent`))
  (cast `GeneralCharacter` OtherActor)
  (`ChaosVehicleMovementComponent.SetThrottleInput` _vehiclemovementcomponent (`self.MaxThrottle`))
  (`ChaosVehicleMovementComponent.SetBrakeInput` _vehiclemovementcomponent 0.0)
  (`ChaosVehicleMovementComponent.SetHandbrakeInput` _vehiclemovementcomponent false)
  (set `self.CanFollowPath` true))

(event `Continue`
  (params (Character :type "GeneralCharacter Object Reference"))
  (bind _vehiclemovementcomponent (`self.VehicleMovementComponent`))
  (set `self.CanFollowPath` true)
  (bind _output_get (set `self.MaxThrottle` 0.4))
  (`ChaosVehicleMovementComponent.SetThrottleInput` _vehiclemovementcomponent _output_get)
  (`ChaosVehicleMovementComponent.SetBrakeInput` _vehiclemovementcomponent 0.0))

(event `Brakeeee`
  (params (Character :type "GeneralCharacter Object Reference"))
  (bind _vehiclemovementcomponent (`self.VehicleMovementComponent`))
  (set `self.CanFollowPath` false)
  (`ChaosVehicleMovementComponent.SetThrottleInput` _vehiclemovementcomponent (`self.MaxThrottle`))
  (`ChaosVehicleMovementComponent.SetBrakeInput` _vehiclemovementcomponent 0.3)
  (`MaterialInstanceDynamic.SetScalarParameterValue` (`self.BackLightMaterial`) "EmissiveIntensity" 50.0)
  (`KismetSystemLibrary.Delay` 0.25)
  (`GameplayStatics.PlaySoundAtLocation` "/Game/Sounds/Files/CarBrake.CarBrake" (`self.K2_GetActorLocation`) (struct) 1.0 1.0 0.0 null null null null))

(event `self.ReceiveBeginPlay`
  (bind _asbp_light (cast `/Game/GeneralBlueprints/BP_Light` (`ChildActorComponent.ChildActor` (`self.CarLight`))))
  (add `/Game/GeneralBlueprints/BP_Light.CharacterEnterLight` _asbp_light (delegate `Brakeeee`))
  (add `/Game/GeneralBlueprints/BP_Light.CharacterLeaveLight` _asbp_light (delegate `Continue`)))

(event `self.ReceiveTick`
  (params (DeltaSeconds :type "Float (single-precision)"))
  (bind _vehiclemovementcomponent (`self.VehicleMovementComponent`))
  (`AudioComponent.SetPitchMultiplier` (`self.EngineSound`) (`KismetMathLibrary.MapRangeClamped` (/ (`ChaosVehicleMovementComponent.GetForwardSpeed` (`self.VehicleMovementComponent`)) 400.0) 0.0 1.0 1.0 1.75))
  (if (`self.CanFollowPath`)
    (bind (_steering _throttle) (`self.Get Car Params`))
    (`ChaosVehicleMovementComponent.SetSteeringInput` _vehiclemovementcomponent _steering)
    (`ChaosVehicleMovementComponent.SetThrottleInput` _vehiclemovementcomponent _throttle)))

(fn `Get Car Params`
  (returns (Steering :type "Float (double-precision)") (Throttle :type "Float (double-precision)") (Brake :type "Float (double-precision)"))
  (bind _backlightmaterial (`self.BackLightMaterial`))
  (bind _spline (`/Game/GeneralProps/Car/Blueprints/BP_CarPath.Spline` (`self.Path`)))
  (bind _returnvalue (+ (`self.K2_GetActorLocation`) (* (`self.GetActorForwardVector`) (200.0 200.0 200.0))))
  (bind (_returnvalue_roll _returnvalue_pitch _returnvalue_yaw) (`KismetMathLibrary.BreakRotator` (`KismetMathLibrary.NormalizedDeltaRotator` (`KismetMathLibrary.FindLookAtRotation` _returnvalue (`SplineComponent.FindLocationClosestToWorldLocation` _spline (+ _returnvalue (* (`KismetMathLibrary.Normal` (`SplineComponent.FindTangentClosestToWorldLocation` _spline _returnvalue "World")) (`self.TangentScale`))) "World")) (`self.K2_GetActorRotation`))))
  (bind _returnvalue_2 (`KismetMathLibrary.MapRangeClamped` _returnvalue_yaw -90.0 90.0 -1.0 1.0))
  (bind _returnvalue_3 (`KismetMathLibrary.Abs` _returnvalue_2))
  (bind _returnvalue_4 (`KismetMathLibrary.MapRangeClamped` _returnvalue_3 0.0 1.0 (`self.MaxThrottle`) 0.01))
  (if (>= _returnvalue_3 0.5)
    (`MaterialInstanceDynamic.SetScalarParameterValue` _backlightmaterial "EmissiveIntensity" 50.0)
    (return _returnvalue_2 _returnvalue_4 1.0)
    (else
      (`MaterialInstanceDynamic.SetScalarParameterValue` _backlightmaterial "EmissiveIntensity" 2.0)
      (return _returnvalue_2 _returnvalue_4 0.0))))

(fn `UserConstructionScript`
  (bind _returnvalue (`KismetMaterialLibrary.CreateDynamicMaterialInstance` "/Game/GeneralProps/Car/Meshes/CarBackLights_MAT_Inst.CarBackLights_MAT_Inst"))
  (`PrimitiveComponent.SetMaterial` (`self.Mesh`) 7 _returnvalue)
  (set `self.BackLightMaterial` _returnvalue))