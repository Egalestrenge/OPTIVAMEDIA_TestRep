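; Isometric camera that follows the player along a spline, CameraPath, sitting behind the path point along its view axis with a fixed height lift.
; Each tick it eases toward the spline point nearest the player and stores that input key as PositionInSpline.
; A second interpolation on the same tick adds optional ZoomCurve distance sampled at that key.
; The construction script snaps the camera to the offset for PositionInSpline.
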(event `self.ReceiveTick`
  (params (DeltaSeconds :type "Float (single-precision)"))
  (`self.Get Spline Position From Player`)
  (`self.GetZoomAtSplinePosition`))

(fn `Get Spline Position From Player`
  (bind _returnvalue (`SplineComponent.FindLocationClosestToWorldLocation` (`self.CameraPath`) (`self.K2_GetActorLocation` (`GameplayStatics.GetPlayerCharacter` 0)) "World"))
  (`SceneComponent.K2_SetWorldLocation` (`self.CameraComponent`) (`KismetMathLibrary.VInterpTo` (`SceneComponent.K2_GetComponentLocation` (`self.CameraComponent`)) (+ _returnvalue (`KismetMathLibrary.TransformDirection` (`SceneComponent.K2_GetComponentToWorld` (`self.CameraComponent`)) (`KismetMathLibrary.MakeVector` (* (`self.Distance`) -1.0))) (0.0 0.0 300.0)) (`GameplayStatics.GetWorldDeltaSeconds`) 1.0) false false)
  (set `self.PositionInSpline` (`SplineComponent.FindInputKeyClosestToWorldLocation` (`self.CameraPath`) _returnvalue)))

(fn `GetZoomAtSplinePosition`
  (bind _cameracomponent (`self.CameraComponent`))
  (bind _zoomcurve (`self.ZoomCurve`))
  (`/Engine/EditorBlueprintResources/StandardMacros.IsValid` _zoomcurve
    (:`Is Valid`
      (`SceneComponent.K2_SetWorldLocation` _cameracomponent (`KismetMathLibrary.VInterpTo` (`SceneComponent.K2_GetComponentLocation` _cameracomponent) (+ (`SplineComponent.GetLocationAtSplineInputKey` (`self.CameraPath`) (`self.PositionInSpline`) "World") (`KismetMathLibrary.TransformDirection` (`SceneComponent.K2_GetComponentToWorld` (`self.CameraComponent`)) (`KismetMathLibrary.MakeVector` (* (+ (`self.Distance`) (`CurveFloat.GetFloatValue` _zoomcurve (`self.PositionInSpline`))) -1.0))) (0.0 0.0 300.0)) (`GameplayStatics.GetWorldDeltaSeconds`) 1.0) false false))))

(fn `UserConstructionScript`
  (bind _zoomcurve (`self.ZoomCurve`))
  (`/Engine/EditorBlueprintResources/StandardMacros.IsValid` _zoomcurve
    (:`Is Valid`
      (`SceneComponent.K2_SetWorldLocation` (`self.CameraComponent`) (+ (`SplineComponent.GetLocationAtSplineInputKey` (`self.CameraPath`) (`self.PositionInSpline`) "World") (`KismetMathLibrary.TransformDirection` (`SceneComponent.K2_GetComponentToWorld` (`self.CameraComponent`)) (`KismetMathLibrary.MakeVector` (* (+ (`self.Distance`) (`CurveFloat.GetFloatValue` _zoomcurve (`self.PositionInSpline`))) -1.0))) (0.0 0.0 300.0)) false false))
    (:`Is Not Valid`
      (`SceneComponent.K2_SetWorldLocation` (`self.CameraComponent`) (+ (`SplineComponent.GetLocationAtSplineInputKey` (`self.CameraPath`) (`self.PositionInSpline`) "World") (`KismetMathLibrary.TransformDirection` (`SceneComponent.K2_GetComponentToWorld` (`self.CameraComponent`)) (`KismetMathLibrary.MakeVector` (* (`self.Distance`) -1.0))) (0.0 0.0 300.0)) false false))))